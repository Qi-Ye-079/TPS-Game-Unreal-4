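; AI controller for EnemyAI_BP enemies that patrols waypoints and chases the player once found.
; On BeginPlay it caches the controlled pawn, starts a half-second looping timer and begins the patrol.
; The timer polls the pawn's FoundPlayer flag and moves to the player character when it is set.
; Patrol cycles through the pawn's PatrolWayPoints with AIMoveTo, pausing briefly after each arrival and continuing only on success.
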(event Custom|Go%20To%20Next%20Waypoint
  ;[1 1 1] Go to the next waypoint of the Ai
  (AI|AIMoveTo 0 "0, 0, 0" (Utilities|Array|Get(acopy) (Variables|/Script/TpsTutorial.EnemyAI|GetPatrolWayPoints (Variables|Default|GetControlled%20Enemy%20AI%20BP)) (Variables|Default|GetNext%20Waypoint%20Index)) 5e+01 false
    (:OnSuccess
      (Variables|Default|SetNext%20Waypoint%20Index (Math|Integer|%(Integer) (+ (Variables|Default|GetNext%20Waypoint%20Index) 1) (Utilities|Array|Length (Variables|/Script/TpsTutorial.EnemyAI|GetPatrolWayPoints (Variables|Default|GetControlled%20Enemy%20AI%20BP)))))
      (Utilities|FlowControl|Delay 1.0)
      (CallFunction|GotoNextWaypoint))))

(event Custom|Check%20Found%20Player
  ;[1 1 1] Check if a player is found. If found, hunt player
  (if (Variables|/Script/TpsTutorial.EnemyAI|GetFoundPlayer (stale EventBeginPlay _output_get))
    (AI|Navigation|MovetoActor (Game|GetPlayerCharacter 0) 1e+02 true true true 0)))

(event EventBeginPlay
  ;[1 1 1] Set up timer to poll if player is found, and go to next way point at beginning
  (bind _asenemy_ai_bp (Utilities|Casting|CastToEnemyAI_BP (Pawn|GetControlledPawn)))
  (bind _output_get (Variables|Default|SetControlled%20Enemy%20AI%20BP _asenemy_ai_bp))
  (Utilities|Time|SetTimerbyEvent (delegate Custom|Check%20Found%20Player) 0.5 true)
  (CallFunction|GotoNextWaypoint))

(fn ConstructionScript)