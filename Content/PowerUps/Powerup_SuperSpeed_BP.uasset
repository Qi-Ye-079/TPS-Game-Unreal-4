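; Super speed power-up that temporarily triples the walk speed of the first local player's character.
; OnActivated hides the icon mesh and sets the movement component's MaxWalkSpeed to three times GetMaxSpeed.
; OnExpired divides GetMaxSpeed by the same factor and destroys the actor.
; The original speed is not cached, and GetMaxSpeed follows the current movement mode, so restoration depends on the mode at each event.
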(event EventBeginPlay)

(event Collision|EventActorBeginOverlap
  (params (OtherActor :type Actor%20Object%20Reference)))

(event EventTick
  (params (DeltaSeconds :type Float%20%28single-precision%29)))

(event EventOnActivated
  (bind _returnvalue (Game|GetPlayerCharacter 0))
  (bind _returnvalue_2 (Actor|GetComponentbyClass _returnvalue "/Script/Engine.CharacterMovementComponent"))
  (Rendering|SetVisibility (Variables|Default|GetStaticMeshIconComp) false true)
  (Variables|/Script/Engine.CharacterMovementComponent|SetMaxWalkSpeed _returnvalue_2 (* (Class|MovementComponent|GetMaxSpeed _returnvalue_2) 3.0)))

(event EventOnExpired
  (bind _returnvalue (Game|GetPlayerCharacter 0))
  (bind _returnvalue_2 (Actor|GetComponentbyClass _returnvalue "/Script/Engine.CharacterMovementComponent"))
  (Variables|/Script/Engine.CharacterMovementComponent|SetMaxWalkSpeed _returnvalue_2 (/ (Class|MovementComponent|GetMaxSpeed _returnvalue_2) 3.0))
  (Actor|DestroyActor))

(fn ConstructionScript)