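; Health regeneration powerup Blueprint that heals the player over its active duration.
; On activation it hides its icon mesh, and on each powerup tick it heals player 0's TpsHealthComponent by a fixed amount and prints the current health.
; It destroys itself when the powerup expires.
; Healing always targets the first player character, regardless of who picked it up.
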(event EventBeginPlay)

(event Collision|EventActorBeginOverlap
  (params (OtherActor :type Actor%20Object%20Reference)))

(event EventTick
  (params (DeltaSeconds :type Float%20%28single-precision%29)))

(event EventOnPowerupTicked
  (bind _returnvalue (Game|GetPlayerCharacter 0))
  (bind _returnvalue_2 (Actor|GetComponentbyClass _returnvalue "/Script/TpsTutorial.TpsHealthComponent"))
  (Utilities|IsValid _returnvalue_2
    (:Is%20Valid
      (Class|TpsHealthComponent|Heal _returnvalue_2 1e+01)
      (Development|PrintString (Utilities|String|ToString(Float) (Class|TpsHealthComponent|GetCurrentHealth _returnvalue_2))))))

(event EventOnActivated
  (Rendering|SetVisibility (Variables|Default|GetStaticMeshIconComp) false true))

(event EventOnExpired
  (Actor|DestroyActor))

(fn ConstructionScript)