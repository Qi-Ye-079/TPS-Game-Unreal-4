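; Third-person shooter character Blueprint that provides the player's HUD widgets.
; Two custom events create the crosshair and health indicator widgets and add them to the viewport as visible, with no caller in this graph.
; A disconnected weapon spawn-and-attach chain remains as an alternative to the C++ version.
; Tick, overlap and construction script are empty, and the zoom variables are unused here.
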(event Collision|EventActorBeginOverlap
  (params (OtherActor :type Actor%20Object%20Reference)))

(event EventTick
  (params (DeltaSeconds :type Float%20%28single-precision%29)))

(event EventCreateCrosshairWidgetEvent
  ;[1 1 1] Create the cross hair widget for the player
  (bind _returnvalue (UserInterface|CreateWidget "/Game/Blueprints/UI/crosshair_BP.crosshair_BP_C"))
  (UserInterface|Viewport|AddtoViewport _returnvalue 0)
  (Widget|SetVisibility _returnvalue "Visible"))

(event EventCreateHealthIndicatorEvent
  ;[1 1 1] Create the health indicator widget for the player
  (bind _returnvalue (UserInterface|CreateWidget "/Game/Blueprints/UI/HealthIndicator_BP.HealthIndicator_BP_C"))
  (UserInterface|Viewport|AddtoViewport _returnvalue 0)
  (Widget|SetVisibility _returnvalue "Visible"))

(fn ConstructionScript)